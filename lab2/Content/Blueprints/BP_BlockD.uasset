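; BP_BlockD is a block actor that shrinks each time another actor begins overlapping it.
; On overlap it calls the parent handler, then multiplies its current actor scale by a uniform factor just below one, so repeated overlaps compound the shrinkage.
; The construction script only calls its parent, and BeginPlay and Tick are disabled stubs.
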(event EventBeginPlay
  (|CallParentFunction) ; This node is disabled and will not be called.\nDrag off pins to build functionality.
)

(event Collision|EventActorBeginOverlap
  (params (OtherActor :type Actor%20Object%20Reference))
  (|CallParentFunction OtherActor)
  (bind _output_get (Variables|Default|SetSize (Transformation|GetActorScale3D)))
  (bind _output_get_2 (Variables|Default|SetSize (* _output_get "0.900000,0.900000,0.900000")))
  (Transformation|SetActorScale3D _output_get_2))

(event EventTick
  (params (DeltaSeconds :type Float%20%28single-precision%29))
  (|CallParentFunction DeltaSeconds) ; This node is disabled and will not be called.\nDrag off pins to build functionality.
)

(fn ConstructionScript
  (|CallParentFunction))